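; Quest Blueprint "Employment Status", which sends the player to obtain and deliver employability documents via the Fiscal Registry, Notary and General Services.
; It builds an ordered root objective collection with a completion binding, then fills it with go-to and talk-to objectives plus a nested proof-of-employment collection.
; A helper creates talk-to objectives from indexed dialogue tree and NPC arrays.
; The "Go to the Notary" objective targets FiscalRegistry as its destination.
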(event EventBeginPlay
  (|CallParentFunction))

(event Collision|EventActorBeginOverlap
  (params (OtherActor :type Actor%20Object%20Reference)))

(event EventTick
  (params (DeltaSeconds :type Float%20%28single-precision%29)))

(fn ConstructionScript
  (Variables|Default|SetQuestName "Employment Status"))

(fn PopulateObjectives
  (params (RootObjectCollection :type BP%20Obj%20Collection%20Object%20Reference))
  (bind _rootobjectivecollection (CallFunction|GetRootObjectiveCollection))
  (Utilities|FlowControl|Sequence
    (:then_0
      (bind _returnvalue (Game|ConstructObjectfromClass "/Game/QuestSystem/Objectives/BP_OBJ_GoTO.BP_OBJ_GoTO_C" (Variables|Default|GetFiscal%20Registry) "Go to Fiscal Registry"))
      (Default|AddObjective _rootobjectivecollection _returnvalue)
      (CallFunction|AddTalktoObjective 0 0 _rootobjectivecollection "Ask for guidance about the employability conditions declaration"))
    (:then_1
      (bind _returnvalue_2 (Game|ConstructObjectfromClass "/Game/QuestSystem/Objectives/BP_Obj_Collection.BP_Obj_Collection_C" false false "Get Proof of employment (Receipts and Declarations)"))
      (bind _output_get (Variables|Default|SetFillAplicationOBJ _returnvalue_2))
      (Default|AddObjective (CallFunction|GetRootObjectiveCollection) _output_get)
      (bind _returnvalue_3 (Game|ConstructObjectfromClass "/Game/QuestSystem/Objectives/BP_OBJ_GoTO.BP_OBJ_GoTO_C" (Variables|Default|GetFiscal%20Registry) "Go to the Notary "))
      (Default|AddObjective (Variables|Default|GetFillAplicationOBJ) _returnvalue_3)
      (CallFunction|AddTalktoObjective 1 1 (Variables|Default|GetFillAplicationOBJ) "Get a Declaration of Employment and Bank Statements of last 3 payments ")
      (bind _returnvalue_4 (Game|ConstructObjectfromClass "/Game/QuestSystem/Objectives/BP_OBJ_GoTO.BP_OBJ_GoTO_C" (Variables|Default|GetFiscal%20Registry) "Return the Documents  to Fiscal Registry 
"))
      (Default|AddObjective (Variables|Default|GetFillAplicationOBJ) _returnvalue_4))
    (:then_2
      (CallFunction|AddTalktoObjective 2 0 (CallFunction|GetRootObjectiveCollection) "Deliver receipts and declarations to the Fiscal Registry")
      (bind _returnvalue_5 (Game|ConstructObjectfromClass "/Game/QuestSystem/Objectives/BP_OBJ_GoTO.BP_OBJ_GoTO_C" (Variables|Default|GetGeneral%20Services) "Return to General Services"))
      (Default|AddObjective (CallFunction|GetRootObjectiveCollection) _returnvalue_5)
      (CallFunction|AddTalktoObjective 3 2 (CallFunction|GetRootObjectiveCollection) "Deliver application in employability declaration"))))

(fn ConstructRootObjectivecollection
  (bind _returnvalue (Game|ConstructObjectfromClass "/Game/QuestSystem/Objectives/BP_Obj_Collection.BP_Obj_Collection_C" true true "Fetch Employability Conditions"))
  (EventDispatchers|BindEventtoOnRootComplete _returnvalue (EventDispatchers|CreateEvent :!event QuestonComplete))
  (return _returnvalue))

(fn AddTalktoObjective
  (params (Dialogue%20index :type Integer) (NPC%20Index :type Integer) (Add%20To :type BP%20Obj%20Collection%20Object%20Reference) (ObjectiveName :type Text))
  (bind _returnvalue (Game|ConstructObjectfromClass "/Game/QuestSystem/Objectives/BP_OBJ_TalkTo.BP_OBJ_TalkTo_C" (Utilities|Array|Get(acopy) (Variables|Default|GetDialogueTrees) Dialogue%20index) 0 (Utilities|Array|Get(acopy) (Variables|Default|GetDeliverNPC) NPC%20Index) ObjectiveName))
  (Default|AddObjective Add%20To _returnvalue)
  (return))