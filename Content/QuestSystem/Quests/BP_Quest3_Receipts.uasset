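; BP_Quest3_Receipts defines the "Report Earnings and Receipts" quest, sending the player between registries to deliver receipts and gather deduction documents.
; PopulateObjectives builds an ordered tree: Fiscal Registry visit, deduction forms, then return.
; The deduction step nests ordered Civil and Land Registry errands, completable in either order.
; Each errand pairs a destination objective with a TalkTo objective, whose helper picks NPC and dialogue tree by array index.
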(event EventBeginPlay
  (|CallParentFunction) ; This node is disabled and will not be called.\nDrag off pins to build functionality.
)

(event Collision|EventActorBeginOverlap
  (params (OtherActor :type Actor%20Object%20Reference)))

(event EventTick
  (params (DeltaSeconds :type Float%20%28single-precision%29)))

(fn ConstructionScript
  (|CallParentFunction))

(fn PopulateObjectives
  (params (RootObjectCollection :type BP%20Obj%20Collection%20Object%20Reference))
  (bind _rootobjectivecollection (CallFunction|GetRootObjectiveCollection))
  (bind _rootobjectivecollection_2 (CallFunction|GetRootObjectiveCollection))
  (Utilities|FlowControl|Sequence
    (:then_0
      ;[1 1 1] 3.1
      (bind _returnvalue (Game|ConstructObjectfromClass "/Game/QuestSystem/Objectives/BP_OBJ_DeliverFile.BP_OBJ_DeliverFile_C" (Variables|Default|GetFiscal%20Registry) "Go to Fiscal Registry"))
      (Default|AddObjective _rootobjectivecollection _returnvalue)
      (CallFunction|AddTalktoObjective 0 0 _rootobjectivecollection "Deliver the receipts at the Counter"))
    (:then_1
      ;[1 1 1] 3.3
      (bind _returnvalue_2 (Game|ConstructObjectfromClass "/Game/QuestSystem/Objectives/BP_Obj_Collection.BP_Obj_Collection_C" false false "Fill Out the Deduction Forms"))
      (bind _output_get (LocalVariables|SetDeduction%20Collection _returnvalue_2))
      (Default|AddObjective (CallFunction|GetRootObjectiveCollection) _output_get)
      ;[1 0.3615 0.72] 3.3.1
      (bind _returnvalue_3 (Game|ConstructObjectfromClass "/Game/QuestSystem/Objectives/BP_Obj_Collection.BP_Obj_Collection_C" true false "Get civil registration certificate"))
      (bind _output_get_2 (LocalVariables|Set3.3.1 _returnvalue_3))
      (Default|AddObjective (LocalVariables|GetDeduction%20Collection) _output_get_2)
      (bind _returnvalue_4 (Game|ConstructObjectfromClass "/Game/QuestSystem/Objectives/BP_OBJ_DeliverFile.BP_OBJ_DeliverFile_C" (Variables|Default|GetCivilRegistry) "Go to Civil Registry"))
      (Default|AddObjective (LocalVariables|Get3.3.1) _returnvalue_4)
      (CallFunction|AddTalktoObjective 1 1 (LocalVariables|Get3.3.1) "Go to the desk and ask for Civil Registry Certificate"))
    (:then_2
      ;[0.8094 1 0.3379] 3.3.2
      (bind _returnvalue_5 (Game|ConstructObjectfromClass "/Game/QuestSystem/Objectives/BP_Obj_Collection.BP_Obj_Collection_C" true false "Get tax benefits dossier"))
      (bind _output_get_3 (LocalVariables|Set3.3.2 _returnvalue_5))
      (Default|AddObjective (LocalVariables|GetDeduction%20Collection) _output_get_3)
      (bind _returnvalue_6 (Game|ConstructObjectfromClass "/Game/QuestSystem/Objectives/BP_OBJ_DeliverFile.BP_OBJ_DeliverFile_C" (Variables|Default|GetLand%20Registry) "Go to to Land Registry"))
      (Default|AddObjective (LocalVariables|Get3.3.2) _returnvalue_6)
      (CallFunction|AddTalktoObjective 2 2 (LocalVariables|Get3.3.2) "Get the Tax benefits dossier"))
    (:then_3
      (bind _returnvalue_7 (Game|ConstructObjectfromClass "/Game/QuestSystem/Objectives/BP_OBJ_DeliverFile.BP_OBJ_DeliverFile_C" (Variables|Default|GetFiscal%20Registry) "Return  to Fiscal Registry"))
      (Default|AddObjective _rootobjectivecollection_2 _returnvalue_7)
      (CallFunction|AddTalktoObjective 3 0 _rootobjectivecollection_2 "Deliver the Deductions Dossier"))))

(fn ConstructRootObjectivecollection
  (bind _returnvalue (Game|ConstructObjectfromClass "/Game/QuestSystem/Objectives/BP_Obj_Collection.BP_Obj_Collection_C" true true "Report Earnings and Receipts"))
  (EventDispatchers|BindEventtoOnRootComplete _returnvalue (EventDispatchers|CreateEvent :!event QuestonComplete))
  (return _returnvalue))

(fn AddTalktoObjective
  (params (Dialogue%20index :type Integer) (NPC%20Index :type Integer) (Add%20To :type BP%20Obj%20Collection%20Object%20Reference) (ObjectiveName :type Text))
  (bind _returnvalue (Game|ConstructObjectfromClass "/Game/QuestSystem/Objectives/BP_OBJ_TalkTo.BP_OBJ_TalkTo_C" (Utilities|Array|Get(acopy) (Variables|Default|GetDialogue%20Trees) Dialogue%20index) 0 (Utilities|Array|Get(acopy) (Variables|Default|GetNPCs) NPC%20Index) ObjectiveName))
  (Default|AddObjective Add%20To _returnvalue)
  (return))