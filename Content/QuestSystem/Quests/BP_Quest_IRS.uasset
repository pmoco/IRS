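; Quest actor for the "File IRS" quest, which activates on BeginPlay and adds itself to the player character.
; It builds an ordered root objective collection: go to General Services, ask an NPC for directions, then finish each valid quest in NextQuest.
; A helper creates talk-to objectives from indexed NPC and dialogue arrays.
; OnQuestComplete does nothing, as its logic for granting follow-up quests is disconnected.
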(event EventQuestonComplete
  (CallFunction|OnQuestComplete)
  (Default|CallOnQuestCompleted))

(event EventBeginPlay
  (|CallParentFunction)
  (CallFunction|ActivateQuest)
  (bind _asbp_first_person_character (Utilities|Casting|CastToBP_FirstPersonCharacter (Game|GetPlayerCharacter 0)))
  (Default|AddQuest _asbp_first_person_character self))

(fn ConstructionScript
  (|CallParentFunction))

(fn PopulateObjectives
  (params (RootObjectCollection :type BP%20Obj%20Collection%20Object%20Reference))
  (Utilities|FlowControl|Sequence
    (:then_0
      (bind _returnvalue (Game|ConstructObjectfromClass "/Game/QuestSystem/Objectives/BP_OBJ_GoTO.BP_OBJ_GoTO_C" (Variables|Default|GetGeneral%20Services) "Go to the General Services"))
      (Default|AddObjective (CallFunction|GetRootObjectiveCollection) _returnvalue)
      (CallFunction|AddTalktoObjective 0 0 (CallFunction|GetRootObjectiveCollection) " ask for directions to submit your IRS"))
    (:then_1
      (for _array_element (Variables|Default|GetNext%20Quest%20)
        (Utilities|IsValid _array_element
          (:Is%20Valid
            (bind _asbp_first_person_character (Utilities|Casting|CastToBP_FirstPersonCharacter (Game|GetPlayerCharacter 0)))
            (bind _returnvalue_2 (Game|ConstructObjectfromClass "/Game/QuestSystem/Objectives/BP_OBJ_FinishQuest.BP_OBJ_FinishQuest_C" _array_element _asbp_first_person_character (Utilities|Text|FormatText "Deliver {Quest} " (Variables|/Game/QuestSystem/Quests/BP_Quest.BP_Quest_C|GetQuestName _array_element))))
            (Default|AddObjective (CallFunction|GetRootObjectiveCollection) _returnvalue_2)))))))

(fn ConstructRootObjectivecollection
  (bind _returnvalue (Game|ConstructObjectfromClass "/Game/QuestSystem/Objectives/BP_Obj_Collection.BP_Obj_Collection_C" true true "File IRS"))
  (EventDispatchers|BindEventtoOnRootComplete _returnvalue (EventDispatchers|CreateEvent :!event QuestonComplete))
  (return _returnvalue))

(fn OnQuestComplete)

(fn AddTalktoObjective
  (params (Dialogue%20index :type Integer) (NPC%20Index :type Integer) (Add%20To :type BP%20Obj%20Collection%20Object%20Reference) (ObjectiveName :type Text))
  (bind _returnvalue (Game|ConstructObjectfromClass "/Game/QuestSystem/Objectives/BP_OBJ_TalkTo.BP_OBJ_TalkTo_C" (Utilities|Array|Get(acopy) (Variables|Default|GetDialogue%20Trees) Dialogue%20index) 0 (Utilities|Array|Get(acopy) (Variables|Default|GetNPCs) NPC%20Index) ObjectiveName))
  (Default|AddObjective Add%20To _returnvalue)
  (return))