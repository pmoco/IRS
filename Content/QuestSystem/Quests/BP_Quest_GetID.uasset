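; BP_Quest_GetID is the "Renewed ID" quest, which walks the player through renewing an official ID at the accreditation counter.
; It overrides objective setup to build an order-required root collection with a completion callback, then fills it in sequence.
; The steps are a counter visit, a nested collection of application tasks, and a talk objective with Susana.
; All counter steps reuse the deliver-file objective class with the same LampTrigger destination.
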(event EventBeginPlay
  (|CallParentFunction))

(event Collision|EventActorBeginOverlap
  (params (OtherActor :type Actor%20Object%20Reference)))

(event EventTick
  (params (DeltaSeconds :type Float%20%28single-precision%29)))

(fn ConstructionScript
  (Variables|Default|SetQuestName "Renewed ID"))

(fn PopulateObjectives
  (params (RootObjectCollection :type BP%20Obj%20Collection%20Object%20Reference))
  (Utilities|FlowControl|Sequence
    (:then_0
      (bind _returnvalue (Game|ConstructObjectfromClass "/Game/QuestSystem/Objectives/BP_OBJ_DeliverFile.BP_OBJ_DeliverFile_C" (Variables|Default|GetLampTrigger) "Go to the Acreditation Counter"))
      (Default|AddObjective (CallFunction|GetRootObjectiveCollection) _returnvalue))
    (:then_1
      (bind _returnvalue_2 (Game|ConstructObjectfromClass "/Game/QuestSystem/Objectives/BP_Obj_Collection.BP_Obj_Collection_C" false false "Get Aplication for New ID"))
      (bind _output_get (Variables|Default|SetFillAplicationOBJ _returnvalue_2))
      (Default|AddObjective (CallFunction|GetRootObjectiveCollection) _output_get)
      (bind _returnvalue_3 (Game|ConstructObjectfromClass "/Game/QuestSystem/Objectives/BP_OBJ_DeliverFile.BP_OBJ_DeliverFile_C" (Variables|Default|GetLampTrigger) "Get Aplication Form from AC "))
      (Default|AddObjective (Variables|Default|GetFillAplicationOBJ) _returnvalue_3)
      (bind _returnvalue_4 (Game|ConstructObjectfromClass "/Game/QuestSystem/Objectives/BP_OBJ_DeliverFile.BP_OBJ_DeliverFile_C" (Variables|Default|GetLampTrigger) "Fill and Sign Aplication in AC"))
      (Default|AddObjective (Variables|Default|GetFillAplicationOBJ) _returnvalue_4)
      (bind _returnvalue_5 (Game|ConstructObjectfromClass "/Game/QuestSystem/Objectives/BP_OBJ_DeliverFile.BP_OBJ_DeliverFile_C" (Variables|Default|GetLampTrigger) "Take a photo in AC "))
      (Default|AddObjective (Variables|Default|GetFillAplicationOBJ) _returnvalue_5)
      (bind _returnvalue_6 (Game|ConstructObjectfromClass "/Game/QuestSystem/Objectives/BP_OBJ_DeliverFile.BP_OBJ_DeliverFile_C" (Variables|Default|GetLampTrigger) "Deliver  Aplication in AC"))
      (Default|AddObjective (Variables|Default|GetFillAplicationOBJ) _returnvalue_6))
    (:then_2
      (bind _returnvalue_7 (Game|ConstructObjectfromClass "/Game/QuestSystem/Objectives/BP_OBJ_TalkTo.BP_OBJ_TalkTo_C" (Variables|Default|GetDialogue) 0 (Variables|Default|GetDeliverNPC) "Go talk to susana to deliver ID"))
      (Default|AddObjective (CallFunction|GetRootObjectiveCollection) _returnvalue_7))))

(fn ConstructRootObjectivecollection
  (bind _returnvalue (Game|ConstructObjectfromClass "/Game/QuestSystem/Objectives/BP_Obj_Collection.BP_Obj_Collection_C" true true "Renew Official ID"))
  (EventDispatchers|BindEventtoOnRootComplete _returnvalue (EventDispatchers|CreateEvent :!event QuestonComplete))
  (return _returnvalue))