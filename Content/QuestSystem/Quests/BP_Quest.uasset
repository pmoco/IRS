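; Base quest Blueprint that defines the lifecycle of a quest built around a root objective collection.
; On BeginPlay it constructs the root collection, populates its objectives and activates it.
; Construction and population are template-method hooks for child quests; the base versions only print errors.
; QuestOnComplete prints a completion message and fires the OnQuestCompleted dispatcher, and a getter exposes the root collection.
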(event Custom|QuestOnComplete
  (Development|PrintText "Completed Quest ")
  (Default|CallOnQuestCompleted))

(event EventBeginPlay
  (bind _rootcollection (Private|ConstructRootObjectivecollection))
  (bind _output_get (Variables|Private|SetRootObjectiveCollection _rootcollection))
  (Private|PopulateObjectives _output_get)
  (Default|ActivateObjective (Variables|Private|GetRootObjectiveCollection)))

(fn ConstructionScript)

(fn ConstructRootObjectivecollection
  (Development|PrintString "Error: CreateRootObjectiveCOllection for base class!" true true "(R=1.000000,G=0.000000,B=0.016751,A=1.000000)")
  (return 0))

(fn PopulateObjectives
  (params (RootObjectCollection :type BP%20Obj%20Collection%20Object%20Reference))
  (Development|PrintString "Error: PopulateObjectives called  for base class!" true true "(R=1.000000,G=0.000000,B=0.016751,A=1.000000)"))

(fn GetRootObjectiveCollection
  (return (Variables|Private|GetRootObjectiveCollection)))