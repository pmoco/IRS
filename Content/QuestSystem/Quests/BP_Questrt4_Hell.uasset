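; BP_Questrt4_Hell is the "Income Declaration" quest, a bureaucratic errand chain between registries, offices and NPCs to obtain and deliver income declarations.
; PopulateObjectives builds a nested tree of collection, GoTo and TalkTo objectives under an ordered root, with some collections order-required.
; National Income Declaration builds the national branch, and AddTalkToObjective pairs dialogue trees with NPCs by index.
; The Notary steps attach to the proof-of-address collection, leaving the investments collection empty.
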(event EventBeginPlay
  (|CallParentFunction) ; This node is disabled and will not be called.\nDrag off pins to build functionality.
)

(event Collision|EventActorBeginOverlap
  (params (OtherActor :type Actor%20Object%20Reference)))

(event EventTick
  (params (DeltaSeconds :type Float%20%28single-precision%29)))

(fn ConstructionScript
  (Variables|Default|SetQuestName "Income Declaration"))

(fn PopulateObjectives
  (params (RootObjectCollection :type BP%20Obj%20Collection%20Object%20Reference))
  (Utilities|FlowControl|Sequence
    (:then_0
      (CallFunction|AddTalktoObjective 0 0 (CallFunction|GetRootObjectiveCollection) "Learn about income sources at the Fiscal Registry"))
    (:then_1
      (bind _returnvalue (Game|ConstructObjectfromClass "/Game/QuestSystem/Objectives/BP_Obj_Collection.BP_Obj_Collection_C" false false "Get Income Declarations"))
      (bind _output_get (LocalVariables|SetIncomeDeclarations _returnvalue))
      (Default|AddObjective (CallFunction|GetRootObjectiveCollection) _output_get)
      (Utilities|FlowControl|Sequence
        (:then_0
          (|NationalIncomeDeclaration (LocalVariables|GetIncomeDeclarations)))
        (:then_1
          (bind _returnvalue_2 (Game|ConstructObjectfromClass "/Game/QuestSystem/Objectives/BP_Obj_Collection.BP_Obj_Collection_C" true false "Get International  income declaration"))
          (bind _output_get_2 (LocalVariables|SetInternationalDeclaration _returnvalue_2))
          (Default|AddObjective (LocalVariables|GetIncomeDeclarations) _output_get_2)
          (bind _returnvalue_3 (Game|ConstructObjectfromClass "/Game/QuestSystem/Objectives/BP_OBJ_GoTO.BP_OBJ_GoTO_C" (Variables|Default|GetArchive) "Go to the Archive"))
          (Default|AddObjective (LocalVariables|GetInternationalDeclaration) _returnvalue_3)
          (CallFunction|AddTalktoObjective 3 1 (LocalVariables|GetInternationalDeclaration) "Receive Transfers from abroad extract"))
        (:then_2
          (bind _returnvalue_4 (Game|ConstructObjectfromClass "/Game/QuestSystem/Objectives/BP_OBJ_GoTO.BP_OBJ_GoTO_C" (Variables|Default|GetFiscal%20Registry) "Return to Fiscal Registry"))
          (Default|AddObjective (LocalVariables|GetIncomeDeclarations) _returnvalue_4)
          (CallFunction|AddTalktoObjective 3 1 (LocalVariables|GetIncomeDeclarations) "Receive Transfers from abroad extract"))))
    (:then_2
      (bind _returnvalue_5 (Game|ConstructObjectfromClass "/Game/QuestSystem/Objectives/BP_OBJ_GoTO.BP_OBJ_GoTO_C" (Variables|Default|GetGeneral%20Registry) "Return to General Services"))
      (Default|AddObjective (CallFunction|GetRootObjectiveCollection) _returnvalue_5)
      (CallFunction|AddTalktoObjective 3 1 (CallFunction|GetRootObjectiveCollection) "Deliver “other income sources declaration” "))))

(fn ConstructRootObjectivecollection
  (bind _returnvalue (Game|ConstructObjectfromClass "/Game/QuestSystem/Objectives/BP_Obj_Collection.BP_Obj_Collection_C" true true "Declare other income sources declaration"))
  (EventDispatchers|BindEventtoOnRootComplete _returnvalue (EventDispatchers|CreateEvent :!event QuestonComplete))
  (return _returnvalue))

(fn AddTalktoObjective
  (params (Dialogue%20index :type Integer) (NPC%20Index :type Integer) (Add%20To :type BP%20Obj%20Collection%20Object%20Reference) (ObjectiveName :type Text))
  (bind _returnvalue (Game|ConstructObjectfromClass "/Game/QuestSystem/Objectives/BP_OBJ_TalkTo.BP_OBJ_TalkTo_C" (Utilities|Array|Get(acopy) (Variables|Default|GetDialogue%20Trees) Dialogue%20index) 0 (Utilities|Array|Get(acopy) (Variables|Default|GetNPCs) NPC%20Index) ObjectiveName))
  (Default|AddObjective Add%20To _returnvalue)
  (return))