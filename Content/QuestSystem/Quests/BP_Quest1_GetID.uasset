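; Quest Blueprint for "Renewed ID", in which the player renews an official ID by visiting service locations and talking to NPCs.
; It builds an ordered root objective collection, then fills it with go-to and talk-to objectives around a nested ordered collection for the application steps.
; A helper creates each talk-to objective, taking its dialogue tree and NPC from arrays by index.
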(event EventBeginPlay
  (|CallParentFunction))

(event Collision|EventActorBeginOverlap
  (params (OtherActor :type Actor%20Object%20Reference)))

(event EventTick
  (params (DeltaSeconds :type Float%20%28single-precision%29)))

(fn ConstructionScript
  (Variables|Default|SetQuestName "Renewed ID"))

(fn PopulateObjectives
  (params (RootObjectCollection :type BP%20Obj%20Collection%20Object%20Reference))
  (bind _rootobjectivecollection (CallFunction|GetRootObjectiveCollection))
  (Utilities|FlowControl|Sequence
    (:then_0
      (bind _returnvalue (Game|ConstructObjectfromClass "/Game/QuestSystem/Objectives/BP_OBJ_GoTO.BP_OBJ_GoTO_C" (Variables|Default|GetAccreditation%20Counter) "Go to the Acreditation Counter"))
      (Default|AddObjective _rootobjectivecollection _returnvalue)
      (CallFunction|AddTalktoObjective 0 0 _rootobjectivecollection "Find the way to Renew the ID "))
    (:then_1
      (bind _returnvalue_2 (Game|ConstructObjectfromClass "/Game/QuestSystem/Objectives/BP_Obj_Collection.BP_Obj_Collection_C" true false "Get Aplication for New ID"))
      (bind _output_get (Variables|Default|SetFillAplicationOBJ _returnvalue_2))
      (Default|AddObjective (CallFunction|GetRootObjectiveCollection) _output_get)
      (CallFunction|AddTalktoObjective 0 0 (Variables|Default|GetFillAplicationOBJ) "Fill & Sign application")
      (CallFunction|AddTalktoObjective 0 0 (Variables|Default|GetFillAplicationOBJ) "Take a Photo")
      (CallFunction|AddTalktoObjective 0 0 (Variables|Default|GetFillAplicationOBJ) "Deliver the aplication in Accreditation Counter"))
    (:then_2
      (bind _returnvalue_3 (Game|ConstructObjectfromClass "/Game/QuestSystem/Objectives/BP_OBJ_GoTO.BP_OBJ_GoTO_C" (Variables|Default|GetGeneralServices) "Go to the Acreditation Counter"))
      (Default|AddObjective (CallFunction|GetRootObjectiveCollection) _returnvalue_3)
      (CallFunction|AddTalktoObjective 0 0 (CallFunction|GetRootObjectiveCollection) "Present legible identification"))))

(fn ConstructRootObjectivecollection
  (bind _returnvalue (Game|ConstructObjectfromClass "/Game/QuestSystem/Objectives/BP_Obj_Collection.BP_Obj_Collection_C" true true "Renew Official ID"))
  (EventDispatchers|BindEventtoOnRootComplete _returnvalue (EventDispatchers|CreateEvent :!event QuestonComplete))
  (return _returnvalue))

(fn AddTalktoObjective
  (params (Dialogue%20index :type Integer) (NPC%20Index :type Integer) (Add%20To :type BP%20Obj%20Collection%20Object%20Reference) (ObjectiveName :type Text))
  (bind _returnvalue (Game|ConstructObjectfromClass "/Game/QuestSystem/Objectives/BP_OBJ_TalkTo.BP_OBJ_TalkTo_C" (Utilities|Array|Get(acopy) (Variables|Default|GetDialogueTrees) Dialogue%20index) 0 (Utilities|Array|Get(acopy) (Variables|Default|GetDeliverNPC) NPC%20Index) ObjectiveName))
  (Default|AddObjective Add%20To _returnvalue)
  (return))