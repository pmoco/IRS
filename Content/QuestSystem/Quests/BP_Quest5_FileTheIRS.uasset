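; Quest Blueprint for "File the IRS declaration", an errand quest between the Archive, General Services and the Accreditation counter.
; It builds a tree of ordered objective collections: obtain and deliver last year's declaration, pay the invoice via an IBAN certificate, then receive the current declaration.
; GoTo objectives supply destinations, while a helper creates TalkTo objectives from indexed NPC and dialogue-tree arrays.
; The root collection binds an event to its completion.
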(event EventBeginPlay
  (|CallParentFunction) ; This node is disabled and will not be called.\nDrag off pins to build functionality.
)

(event Collision|EventActorBeginOverlap
  (params (OtherActor :type Actor%20Object%20Reference)))

(event EventTick
  (params (DeltaSeconds :type Float%20%28single-precision%29)))

(fn ConstructionScript
  (Variables|Default|SetQuestName "IRS"))

(fn PopulateObjectives
  (params (RootObjectCollection :type BP%20Obj%20Collection%20Object%20Reference))
  (Utilities|FlowControl|Sequence
    (:then_0
      (bind _returnvalue (Game|ConstructObjectfromClass "/Game/QuestSystem/Objectives/BP_Obj_Collection.BP_Obj_Collection_C" true false "Get declaration of the previous year's IRS"))
      (bind _output_get (LocalVariables|SetPrevious%20IRS _returnvalue))
      (Default|AddObjective (CallFunction|GetRootObjectiveCollection) _output_get)
      (Utilities|FlowControl|Sequence
        (:then_0
          (bind _returnvalue_2 (Game|ConstructObjectfromClass "/Game/QuestSystem/Objectives/BP_OBJ_GoTO.BP_OBJ_GoTO_C" (Variables|Default|GetArchive) "Go  to the Archive"))
          (Default|AddObjective (LocalVariables|GetPrevious%20IRS) _returnvalue_2)
          (CallFunction|AddTalktoObjective 0 0 (LocalVariables|GetPrevious%20IRS) "Receive declaration of the previous year's IRS"))
        (:then_1
          (bind _returnvalue_3 (Game|ConstructObjectfromClass "/Game/QuestSystem/Objectives/BP_OBJ_GoTO.BP_OBJ_GoTO_C" (Variables|Default|GetGeneral%20Services) "Return to General Services"))
          (Default|AddObjective (LocalVariables|GetPrevious%20IRS) _returnvalue_3)
          (CallFunction|AddTalktoObjective 1 1 (LocalVariables|GetPrevious%20IRS) "Deliver declaration of the previous year's IRS"))))
    (:then_1
      (bind _returnvalue_4 (Game|ConstructObjectfromClass "/Game/QuestSystem/Objectives/BP_Obj_Collection.BP_Obj_Collection_C" true false "Pay the Invoice"))
      (bind _output_get_2 (LocalVariables|SetInvoice _returnvalue_4))
      (Default|AddObjective (CallFunction|GetRootObjectiveCollection) _output_get_2)
      (bind _returnvalue_5 (Game|ConstructObjectfromClass "/Game/QuestSystem/Objectives/BP_OBJ_GoTO.BP_OBJ_GoTO_C" (Variables|Default|GetAcreditation%20Counter) "Go to Accreditation counter"))
      (Default|AddObjective (LocalVariables|GetInvoice) _returnvalue_5)
      (CallFunction|AddTalktoObjective 2 2 (LocalVariables|GetInvoice) "Get yout IBAN certificate")
      (bind _returnvalue_6 (Game|ConstructObjectfromClass "/Game/QuestSystem/Objectives/BP_OBJ_GoTO.BP_OBJ_GoTO_C" (Variables|Default|GetGeneral%20Services) "Return to General Services"))
      (Default|AddObjective (LocalVariables|GetInvoice) _returnvalue_6))
    (:then_2
      (CallFunction|AddTalktoObjective 3 1 (CallFunction|GetRootObjectiveCollection) "Deliver IBAN and Recieve the Current IRS declaration"))))

(fn ConstructRootObjectivecollection
  (bind _returnvalue (Game|ConstructObjectfromClass "/Game/QuestSystem/Objectives/BP_Obj_Collection.BP_Obj_Collection_C" true true "File the IRS declaration"))
  (EventDispatchers|BindEventtoOnRootComplete _returnvalue (EventDispatchers|CreateEvent :!event QuestonComplete))
  (return _returnvalue))

(fn AddTalktoObjective
  (params (Dialogue%20index :type Integer) (NPC%20Index :type Integer) (Add%20To :type BP%20Obj%20Collection%20Object%20Reference) (ObjectiveName :type Text))
  (bind _returnvalue (Game|ConstructObjectfromClass "/Game/QuestSystem/Objectives/BP_OBJ_TalkTo.BP_OBJ_TalkTo_C" (Utilities|Array|Get(acopy) (Variables|Default|GetDialogue%20Trees) Dialogue%20index) 0 (Utilities|Array|Get(acopy) (Variables|Default|GetNPCs) NPC%20Index) ObjectiveName))
  (Default|AddObjective Add%20To _returnvalue)
  (return))