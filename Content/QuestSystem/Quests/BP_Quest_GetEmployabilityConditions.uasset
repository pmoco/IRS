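; Quest Blueprint "Employment Status", which sends the player to fetch employability conditions.
; It overrides quest hooks to build an ordered root objective collection with a completion binding and populate it with objectives.
; Only one objective is live, a deliver-file step to the Fiscal Registry targeting LampTrigger.
; Further deliver-file steps, including a nested proof-of-employment collection covering notary, declaration and bank statements, are left unwired and never run.
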(event EventBeginPlay
  (|CallParentFunction))

(event Collision|EventActorBeginOverlap
  (params (OtherActor :type Actor%20Object%20Reference)))

(event EventTick
  (params (DeltaSeconds :type Float%20%28single-precision%29)))

(fn ConstructionScript
  (Variables|Default|SetQuestName "Employment Status"))

(fn PopulateObjectives
  (params (RootObjectCollection :type BP%20Obj%20Collection%20Object%20Reference))
  (Utilities|FlowControl|Sequence
    (:then_0
      (bind _returnvalue (Game|ConstructObjectfromClass "/Game/QuestSystem/Objectives/BP_OBJ_DeliverFile.BP_OBJ_DeliverFile_C" (Variables|Default|GetLampTrigger) "Go to Fiscal Registry"))
      (Default|AddObjective (CallFunction|GetRootObjectiveCollection) _returnvalue))))

(fn ConstructRootObjectivecollection
  (bind _returnvalue (Game|ConstructObjectfromClass "/Game/QuestSystem/Objectives/BP_Obj_Collection.BP_Obj_Collection_C" true true "Fetch Employability Conditions"))
  (EventDispatchers|BindEventtoOnRootComplete _returnvalue (EventDispatchers|CreateEvent :!event QuestonComplete))
  (return _returnvalue))