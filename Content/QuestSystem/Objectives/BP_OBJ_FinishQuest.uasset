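; BP_OBJ_FinishQuest is a quest objective that completes when another quest, QuestToListen, is finished.
; On activation it adds that quest to the character, prints a notice with its name, binds to its completion event and activates it.
; When that quest completes, it unbinds, sets ReachedDestination as its completion flag and broadcasts OnCompleted, allowing quests to nest inside objectives.
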(event Custom|QuestDone
  (EventDispatchers|UnbindEventfromOnQuestCompleted (Variables|Default|GetQuestToListen) (delegate Custom|QuestDone))
  (Variables|Default|SetReached%20Destination%20 true)
  (Default|CallOnCompleted self))

(event EventActivateObjective
  (bind _questtolisten (Variables|Default|GetQuestToListen))
  (|CallParentFunction)
  (|AddQuestToPlayer)
  (EventDispatchers|BindEventtoOnQuestCompleted _questtolisten (delegate Custom|QuestDone))
  (Default|ActivateQuest _questtolisten))

(fn GetItsComplete
  (return (Variables|Default|GetReached%20Destination%20)))