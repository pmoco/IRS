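; Quest objective that completes when the first-person player character reaches a destination actor.
; On activation it runs the parent logic, then binds to the Destination's begin-overlap event.
; An overlap by BP_FirstPersonCharacter sets ReachedDestination, unbinds the event, prints a debug message and calls OnCompleted, a step marked as needing a fix.
; GetItsComplete reports completion from the ReachedDestination flag.
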(event Custom|OnActorBeginOverlap_Event
  (params (OverlappedActor :type Actor%20Object%20Reference) (OtherActor :type Actor%20Object%20Reference))
  (Utilities|Casting|CastToBP_FirstPersonCharacter OtherActor)
  (Variables|Default|SetReached%20Destination%20 true)
  (Collision|UnbindEventfromOnActorBeginOverlap (Variables|Default|GetDestination) (delegate Custom|OnActorBeginOverlap_Event))
  (Development|PrintString 0 "Ive reached destination" true true "(R=0.000000,G=0.000000,B=0.000000,A=1.000000)")
  ;[1 1 1] NEED TO FIX
  (Default|CallOnCompleted self))

(event EventActivateObjective
  (|CallParentFunction)
  (EventDispatchers|AssignOnActorBeginOverlap (Variables|Default|GetDestination) (delegate Custom|OnActorBeginOverlap_Event)))

(fn GetItsComplete
  (return (Variables|Default|GetReached%20Destination%20)))