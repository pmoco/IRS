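; Quest objective that completes when a dialogue with the target NPC (the DonaSusana reference) ends.
; On activation it gets the target's NPC_AI controller, binds to its end-of-dialogue event and swaps in the objective's dialogue tree, caching the original.
; When dialogue ends it restores that tree, marks itself complete, unbinds and fires OnCompleted, a step flagged as needing a fix.
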(event Custom|DialogueCompleted
  (CallFunction|DeactivateNPC)
  (EventDispatchers|UnbindEventfromEndDialogue (Variables|Default|GetNPC) (delegate Custom|DialogueCompleted))
  (Development|PrintString 0 (Utilities|String|ToString(Text) (Utilities|Text|FormatText "Talked to {Atendee}" (Utilities|GetDisplayName (Variables|Default|GetDonaSusana)))) true true "(R=0.000000,G=0.000000,B=0.000000,A=1.000000)")
  ;[1 1 1] NEED TO FIX
  (Default|CallOnCompleted self))

(event EventActivateObjective
  (|CallParentFunction)
  (bind _asnpc_ai (Utilities|Casting|CastToNPC_AI (Pawn|GetController (Variables|Default|GetDonaSusana))))
  (bind _output_get (Variables|Default|SetNPC _asnpc_ai))
  (EventDispatchers|BindEventtoEndDialogue _output_get (delegate Custom|DialogueCompleted))
  (CallFunction|ActivateNPC))

(fn GetItsComplete
  (return (Variables|Default|GetObjectiveCompleted)))

(fn ActivateNPC
  (if (Utilities|IsValid (Variables|Default|GetReturnDialogue))
    _
    (else
      (Variables|Default|SetReturnDialogue (Variables|/Game/Characters/DonaSusana/NPC_AI.NPC_AI_C|GetDialogue%20Tree (Variables|Default|GetNPC)))))
  (Variables|/Game/Characters/DonaSusana/NPC_AI.NPC_AI_C|SetDialogue%20Tree (Variables|Default|GetNPC) (Variables|Default|GetDialogue)))

(fn DeactivateNPC
  (Variables|/Game/Characters/DonaSusana/NPC_AI.NPC_AI_C|SetDialogue%20Tree (Variables|Default|GetNPC) (Variables|Default|GetReturnDialogue))
  (Variables|Default|SetObjectiveCompleted true))